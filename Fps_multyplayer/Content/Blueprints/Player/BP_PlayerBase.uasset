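; BP_PlayerBase is a base player Blueprint that handles Enhanced Input movement and camera look.
; On BeginPlay it prints a debug string, gets the player controller through a message call on its controller, and adds the IMS_Default mapping context.
; IA_Movement drives movement along the actor's forward and right vectors, while IA_Look feeds controller yaw and pitch input.
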(event `self.ReceiveBeginPlay`
  ;[0.03614 1 0] Input Mapping Context
  (`KismetSystemLibrary.PrintString` "Hello")
  (bind _playercontroller (message `/Game/Blueprints/Interfaces/INT_PlayerController.GetPlayerControllerRef` (`self.GetController`)))
  (`EnhancedInputSubsystemInterface.AddMappingContext` (pcsubsystem `EnhancedInputLocalPlayerSubsystem` _playercontroller) "/Game/Blueprints/Player/Input/IMS_Default.IMS_Default" 0 (struct)))

(event `EnhancedInput|/Game/Blueprints/Player/Input/IA_Movement`
  (params (ActionValue :type "Vector2D Structure") (ElapsedSeconds :type "Float (double-precision)") (TriggeredSeconds :type "Float (double-precision)") (InputAction :type "InputAction Object Reference" :default "/Game/Blueprints/Player/Input/IA_Movement.IA_Movement"))
  (bind (_x _y) (`KismetMathLibrary.BreakVector2D` ActionValue))
  ;[0.03614 1 0] MOVEMENT
  (:`Triggered`
    (`self.AddMovementInput` (`self.GetActorForwardVector`) _x)
    (`self.AddMovementInput` (`self.GetActorRightVector`) _y)))

(event `EnhancedInput|/Game/Blueprints/Player/Input/IA_Look`
  (params (ActionValue :type "Vector2D Structure") (ElapsedSeconds :type "Float (double-precision)") (TriggeredSeconds :type "Float (double-precision)") (InputAction :type "InputAction Object Reference" :default "/Game/Blueprints/Player/Input/IA_Look.IA_Look"))
  ;[0.03614 1 0] Looking
  (:`Triggered`
    (`self.AddControllerYawInput` ActionValue_X)
    (`self.AddControllerPitchInput` ActionValue_Y)))

(fn `UserConstructionScript`)