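; Game mode for the shooter menu that tracks connected players and syncs player profiles in the lobby.
; When a player starts on the lobby menu map, it registers their controller and triggers lobby menu creation and initial setup.
; Lobby updates can rebuild the profile list from connected controllers and push it to each for name display.
; Logout removes the controller and refreshes the remaining players' lists.
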(event `self.K2_OnLogout`
  (params (ExitingController :type "Controller Object Reference"))
  (bind _asbp_shooter_menu_controller (cast `/Game/FrameWork/BP_shooterMenu_controller` ExitingController))
  (`KismetArrayLibrary.Array_RemoveItem` (`self.All_conectedplayers`) _asbp_shooter_menu_controller)
  (`self.updateLobby` true))

(event `self.HandleStartingNewPlayer`
  (params (NewPlayer :type "PlayerController Object Reference"))
  (bind _returnvalue (`GameplayStatics.GetCurrentLevelName` true))
  (switch `string` _returnvalue
    (:`LobbymenuMap`
      (bind _asbp_shooter_menu_controller (cast `/Game/FrameWork/BP_shooterMenu_controller` NewPlayer))
      (`KismetArrayLibrary.Array_Add` (`self.All_conectedplayers`) _asbp_shooter_menu_controller)
      (`/Game/FrameWork/BP_shooterMenu_controller.Createlobbymenu` _asbp_shooter_menu_controller)
      (`/Game/FrameWork/BP_shooterMenu_controller.Initial_Setup` _asbp_shooter_menu_controller))))

(event `updateLobby`
  (params (playerNames :type Boolean))
  (if playerNames
    (`KismetArrayLibrary.Array_Clear` (`self.All_PlayerProfiles`))
    (for _array_element (`self.All_conectedplayers`)
      (`KismetArrayLibrary.Array_Add` (`self.All_PlayerProfiles`) (`/Game/FrameWork/BP_shooterMenu_controller.Player Profile` _array_element)))
    (for _array_element_2 (`self.All_conectedplayers`)
      (if playerNames
        (`/Game/FrameWork/BP_shooterMenu_controller.UpdatePlayerNames` _array_element_2 (`self.All_PlayerProfiles`))))))

(fn `UserConstructionScript`)