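; Shooter game mode that spawns players at numbered player starts as they join the match.
; On each new player it stores the controller and reads the expected player count and solo flag from the game instance.
; Solo games restart the first controller at start "0" immediately.
; Multiplayer waits until all expected controllers have joined, then after a short delay restarts each at the start named by its join index.
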(event `self.HandleStartingNewPlayer`
  (params (NewPlayer :type "PlayerController Object Reference"))
  (bind _asbp_shotter_player_controller (cast `/Game/FrameWork/BP_shotter_PlayerController` NewPlayer))
  (`KismetArrayLibrary.Array_Add` (`self.All_ConectedControllers`) _asbp_shotter_player_controller)
  (bind _asbp_shooter_gameinstance (cast `/Game/FrameWork/BP_shooter_Gameinstance` (`GameplayStatics.GetGameInstance`)))
  (set `self.Num Conected Players` (`/Game/FrameWork/BP_shooter_Gameinstance.NumConectedPlayers` _asbp_shooter_gameinstance))
  (if (`/Game/FrameWork/BP_shooter_Gameinstance.IsSoloGame` _asbp_shooter_gameinstance)
    (set `self.Num Conected Players` 1)
    (`self.RestartPlayerAtPlayerStart` (`|GetArrayItem` (`self.All_ConectedControllers`)) (`self.K2_FindPlayerStart` null "0"))
    (elif (== (`self.Num Conected Players`) (`KismetArrayLibrary.Array_Length` (`self.All_ConectedControllers`)))
      (`KismetSystemLibrary.Delay` 0.5)
      (for (_array_element _array_index) (`self.All_ConectedControllers`)
        (`self.RestartPlayerAtPlayerStart` _array_element (`self.K2_FindPlayerStart` _array_element (`KismetStringLibrary.Conv_IntToString` _array_index)))))))

(fn `UserConstructionScript`)