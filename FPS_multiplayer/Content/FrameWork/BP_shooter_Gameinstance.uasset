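; Shooter game instance that manages the main menu, solo game start and the persistent player profile.
; Showing the menu creates the widget if needed, switches to UI-only input with cursor, then loads or creates the saved profile and fills the name field.
; Name changes rebuild the profile struct and write it to an SG_PlayerProfile save slot.
; Starting solo sets a flag and opens Map_01.
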(event `Start-soloGame`
  (set `self.IsSoloGame` true)
  (`GameplayStatics.OpenLevel` "Map_01"))

(event `Change-PlayerName`
  (params (PlayerName :type Text))
  (set `self.Player Profile` (make `/Game/SavedData/S_PlayerProfile` PlayerName))
  (`self.SaveProfile`))

(fn `CheckedForSavedProfile`
  (bind _returnvalue (`GameplayStatics.DoesSaveGameExist` (`self.PlayerProfile_Slot`)))
  (if _returnvalue
    (`self.LoadProfile`)
    (else
      (`self.SaveProfile`)))
  (return))

(fn `LoadProfile`
  (bind _returnvalue (`GameplayStatics.LoadGameFromSlot` (`self.PlayerProfile_Slot`)))
  (bind _assg_player_profile (cast `/Game/SavedData/SG_PlayerProfile` _returnvalue))
  (set `self.Player Profile` (`/Game/SavedData/SG_PlayerProfile.PlayerProfile` _assg_player_profile))
  (return))

(fn `SaveProfile`
  (bind _sg_playerprofile (`self.SG_PlayerProfile`))
  (`/Engine/EditorBlueprintResources/StandardMacros.IsValid` (`self.SG_PlayerProfile`)
    (:`Is Valid`
      _)
    (:`Is Not Valid`
      (bind _returnvalue (`GameplayStatics.CreateSaveGameObject` "/Game/SavedData/SG_PlayerProfile.SG_PlayerProfile_C"))
      (set `self.SG_PlayerProfile` _returnvalue)))
  (set `/Game/SavedData/SG_PlayerProfile.PlayerProfile` (`self.Player Profile`) _sg_playerprofile)
  (`GameplayStatics.SaveGameToSlot` _sg_playerprofile (`self.PlayerProfile_Slot`))
  (return))

(fn `UI_ShowMainMenu`
  (bind _returnvalue (`GameplayStatics.GetPlayerController` 0))
  (`/Engine/EditorBlueprintResources/StandardMacros.IsValid` (`self.WB_MainMenu`)
    (:`Is Valid`
      _)
    (:`Is Not Valid`
      (bind _returnvalue_2 (`|CreateWidget` "/Game/Widgets/WB_MainMenu.WB_MainMenu_C" _returnvalue))
      (set `self.WB_MainMenu` _returnvalue_2)))
  (`UserWidget.AddToViewport` (`self.WB_MainMenu`) 0)
  (`WidgetBlueprintLibrary.SetInputMode_UIOnlyEx` _returnvalue null)
  (set `PlayerController.bShowMouseCursor` true _returnvalue)
  (`self.CheckedForSavedProfile`)
  (`EditableText.SetText` (`/Game/Widgets/WB_MainMenu.Input_PlayerName` (`self.WB_MainMenu`)) (`.PalyerName_2_B9189AFD4F534000B923DA985F7C2618` (break `/Game/SavedData/S_PlayerProfile` (`self.Player Profile`))))
  (return))