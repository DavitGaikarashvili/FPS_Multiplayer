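; Player controller for the shooter's menus that shows the lobby UI and handles leaving an online session.
; UiShowlobbymenu creates the WB_LobbyMenu widget only when no valid cached instance exists, then adds it to the viewport.
; The Andclientsession event calls DestroySession and opens MainMenumap from its Then output, without branching on success or failure.
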(event `Andclientsession`
  (`DestroySessionCallbackProxy.DestroySession` self
    (:`then`
      (`GameplayStatics.OpenLevel` "MainMenumap"))))

(fn `Ui_Showlobbymenu`
  (`/Engine/EditorBlueprintResources/StandardMacros.IsValid` (`self.WB_Lobbymenu`)
    (:`Is Valid`
      _)
    (:`Is Not Valid`
      (bind _returnvalue (`|CreateWidget` "/Game/Widgets/WB_LobbyMenu.WB_LobbyMenu_C" self))
      (set `self.WB_Lobbymenu` _returnvalue)))
  (`UserWidget.AddToViewport` (`self.WB_Lobbymenu`) 0)
  (return))

(fn `UserConstructionScript`)