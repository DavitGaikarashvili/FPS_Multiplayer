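; Player hero character Quin, with movement, look, aim-down-sights and pistol firing input.
; Axis inputs drive movement and controller yaw and pitch, while possession calls an event that disables input for the possessing controller.
; ADS sets IsADS locally and, on remote clients, sends it through a server event.
; Firing plays muzzle flash and sound, then runs a debug-drawn line trace from the muzzle socket, leaving the hit unused.
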(event `self.ReceivePossessed`
  (params (NewController :type "Controller Object Reference"))
  (`self.DisableAllInput` (cast `PlayerController` NewController :!pure true)))

(event `DisableAllInput`
  (params (PlayerController :type "PlayerController Object Reference"))
  (`self.DisableInput` PlayerController))

(event `InputAxis|turn`
  (params (AxisValue :type "Float (single-precision)"))
  (`self.AddControllerYawInput` AxisValue))

(event `InputAxis|MoveFoward`
  (params (AxisValue :type "Float (single-precision)"))
  (`self.AddMovementInput` (`self.GetActorForwardVector`) AxisValue))

(event `InputAxis|lookUp`
  (params (AxisValue :type "Float (single-precision)"))
  (`self.AddControllerPitchInput` AxisValue))

(event `InputAxis|MoveRight`
  (params (AxisValue :type "Float (single-precision)"))
  (`self.AddMovementInput` (`self.GetActorRightVector`) AxisValue))

(event `InputAction|ADS`
  (params (Key :type "Key Structure"))
  (:`Pressed`
    (`/Engine/EditorBlueprintResources/ActorMacros.Switch Has Authority`
      (:`Authority`
        _)
      (:`Remote`
        (`self.Srv_setisads` true)))
    (set `self.IsADS` true))
  (:`Released`
    (`/Engine/EditorBlueprintResources/ActorMacros.Switch Has Authority`
      (:`Authority`
        _)
      (:`Remote`
        (`self.Srv_setisads` false)))
    (set `self.IsADS` false)))

(event `Srv_setisads`
  (params (IsADS :type Boolean))
  (set `self.IsADS` IsADS))

(event `InputAction|FireWeapon`
  (params (Key :type "Key Structure"))
  (bind (_returnvalue_location _returnvalue_rotation) (`KismetMathLibrary.BreakTransform` (`SceneComponent.GetSocketTransform` (`self.weaponmesh`) "Muzzle" "RTS_World")))
  (:`Pressed`
    (`GameplayStatics.SpawnEmitterAttached` "/Game/MilitaryWeapSilver/FX/P_Pistol_MuzzleFlash_01.P_Pistol_MuzzleFlash_01" (`self.weaponmesh`) "Muzzle" (0.0 0.0 0.0) (struct) (1.0 1.0 1.0) "SnapToTarget")
    (`GameplayStatics.PlaySound2D` "/Game/MilitaryWeapSilver/Sound/Pistol/Cues/PistolA_Fire_Cue.PistolA_Fire_Cue" 1.0 1.0 0.0 null null)
    (`KismetSystemLibrary.LineTraceSingle` :`Start` _returnvalue_location :`End` (+ _returnvalue_location (* (`KismetMathLibrary.GetForwardVector` _returnvalue_rotation) 100000)) :`TraceChannel` "TraceTypeQuery1" :`DrawDebugType` "ForDuration")))

(fn `UserConstructionScript`)